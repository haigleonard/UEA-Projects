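; Fog of war masking actor whose FogWall mesh can have holes painted into it through a render-target mask.
; BeginPlay creates a canvas render target and feeds it to a dynamic material on the wall as MaskTexture.
; AddFogHole, gated by a visibility check, converts the hit to collision UVs and draws a round polygon there on the mask.
; Tick shows or hides the actor according to its floor's visibility in MyGameStateBase.
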(event Custom|AddFogHole
  (params (HitLocation :type Hit%20Result%20Structure))
  (bind _uv (Class|GameplayStatics|FindCollisionUV HitLocation))
  (bind _masktexture (Variables|Default|GetMaskTexture))
  (bind (_x _y) (Math|Vector2D|BreakVector2D _uv))
  (bind (_width _height) (Class|CanvasRenderTarget2D|GetSize _masktexture))
  (bind _returnvalue (Class|FogActor|GetVisibility))
  (if _returnvalue
    (bind (_canvas _size _context) (Rendering|BeginDrawCanvastoRenderTarget _masktexture))
    (Class|Canvas|DrawPolygon _canvas 0 (Math|Vector2D|MakeVector2D (* _width _x) (* _height _y)) "(X=50.000000,Y=50.000000)" 12 "(R=1.000000,G=1.000000,B=1.000000,A=1.000000)")
    (Rendering|EndDrawCanvastoRenderTarget _context)))

(event EventBeginPlay
  (bind _returnvalue (CanvasRenderTarget2D|CreateCanvasRenderTarget2D "/Script/Engine.CanvasRenderTarget2D" 512 512))
  (Variables|Default|SetMaskTexture _returnvalue)
  (bind _returnvalue_2 (Rendering|Material|CreateDynamicMaterialInstance (Variables|Default|GetFogWall) 0 "/Game/FogOfWar/MaskingMat.MaskingMat" :!class /Script/Engine.PrimitiveComponent))
  (bind _output_get (Variables|Default|SetDynamicMaterial _returnvalue_2))
  (Rendering|Material|SetTextureParameterValue _output_get "MaskTexture" (Variables|Default|GetMaskTexture))
  (Rendering|Material|SetMaterial (Variables|Default|GetFogWall) 0 (Variables|Default|GetDynamicMaterial)))

(event Collision|EventActorBeginOverlap
  (params (OtherActor :type Actor%20Object%20Reference)))

(event EventTick
  (params (DeltaSeconds :type Float%20%28single-precision%29))
  (bind _asmy_game_state_base (Utilities|Casting|CastToMyGameStateBase (Game|GetGameState)))
  (bind _returnvalue (Class|MyGameStateBase|GetFloorVisibility _asmy_game_state_base (Variables|Default|GetfloorNumber)))
  (if _returnvalue
    (Rendering|SetActorHiddenInGame false)
    (else
      (Rendering|SetActorHiddenInGame true))))

(fn ConstructionScript)