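; Bomb puzzle light that shows a symbol and toggles between red and green, with the actor label (Symbol 1–4) selecting its slot.
; One second after BeginPlay it sets the symbol material from BombController's SymArray.
; Clicking its meshes flips the light and writes the state to the controller's SymbolLights array.
; Tick also toggles it on every frame that MotionControllerPawn's Hit matches the actor label.
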(event OnClicked(StaticMeshComponent)
  (params (TouchedComponent :type Primitive%20Component%20Object%20Reference) (ButtonPressed :type Key%20Structure))
  (bind _returnvalue (Class|Actor|GetActorLabel))
  (bind _returnvalue_2 (Game|GetPlayerController 0))
  (bind _staticmeshcomponent (Variables|Debug|GetStaticMeshComponent))
  (if (Variables|Default|GetRed)
    (Rendering|Material|SetMaterial _staticmeshcomponent 0 "/Game/Bomb/BombParts/Materials/green_Mat.green_Mat")
    (Variables|Default|SetRed false)
    (bind _asbomb_controller (Utilities|Casting|CastToBombController _returnvalue_2))
    (switch string _returnvalue
      (:Symbol1
        (Utilities|Array|SetArrayElem (Variables|/Game/Bomb/BombController.BombController_C|GetSymbolLights _asbomb_controller) 0 true))
      (:Symbol2
        (Utilities|Array|SetArrayElem (Variables|/Game/Bomb/BombController.BombController_C|GetSymbolLights _asbomb_controller) 1 true))
      (:Symbol3
        (Utilities|Array|SetArrayElem (Variables|/Game/Bomb/BombController.BombController_C|GetSymbolLights _asbomb_controller) 2 true))
      (:Symbol4
        (Utilities|Array|SetArrayElem (Variables|/Game/Bomb/BombController.BombController_C|GetSymbolLights _asbomb_controller) 3 true)))
    (else
      (Rendering|Material|SetMaterial _staticmeshcomponent 0 "/Game/Bomb/BombParts/Materials/red_Mat.red_Mat")
      (Variables|Default|SetRed true)
      (bind _asbomb_controller_2 (Utilities|Casting|CastToBombController _returnvalue_2))
      (switch string _returnvalue
        (:Symbol1
          (Utilities|Array|SetArrayElem (Variables|/Game/Bomb/BombController.BombController_C|GetSymbolLights _asbomb_controller_2) 0 false))
        (:Symbol2
          (Utilities|Array|SetArrayElem (Variables|/Game/Bomb/BombController.BombController_C|GetSymbolLights _asbomb_controller_2) 1 false))
        (:Symbol3
          (Utilities|Array|SetArrayElem (Variables|/Game/Bomb/BombController.BombController_C|GetSymbolLights _asbomb_controller_2) 2 false))
        (:Symbol4
          (Utilities|Array|SetArrayElem (Variables|/Game/Bomb/BombController.BombController_C|GetSymbolLights _asbomb_controller_2) 3 false))))))

(event OnClicked(StaticMesh)
  (params (TouchedComponent :type Primitive%20Component%20Object%20Reference) (ButtonPressed :type Key%20Structure))
  (bind _returnvalue (Class|Actor|GetActorLabel))
  (bind _returnvalue_2 (Game|GetPlayerController 0))
  (bind _staticmeshcomponent (Variables|Debug|GetStaticMeshComponent))
  (if (Variables|Default|GetRed)
    (Rendering|Material|SetMaterial _staticmeshcomponent 0 "/Game/Bomb/BombParts/Materials/green_Mat.green_Mat")
    (Variables|Default|SetRed false)
    (bind _asbomb_controller (Utilities|Casting|CastToBombController _returnvalue_2))
    (switch string _returnvalue
      (:Symbol1
        (Utilities|Array|SetArrayElem (Variables|/Game/Bomb/BombController.BombController_C|GetSymbolLights _asbomb_controller) 0 true))
      (:Symbol2
        (Utilities|Array|SetArrayElem (Variables|/Game/Bomb/BombController.BombController_C|GetSymbolLights _asbomb_controller) 1 true))
      (:Symbol3
        (Utilities|Array|SetArrayElem (Variables|/Game/Bomb/BombController.BombController_C|GetSymbolLights _asbomb_controller) 2 true))
      (:Symbol4
        (Utilities|Array|SetArrayElem (Variables|/Game/Bomb/BombController.BombController_C|GetSymbolLights _asbomb_controller) 3 true)))
    (else
      (Rendering|Material|SetMaterial _staticmeshcomponent 0 "/Game/Bomb/BombParts/Materials/red_Mat.red_Mat")
      (Variables|Default|SetRed true)
      (bind _asbomb_controller_2 (Utilities|Casting|CastToBombController _returnvalue_2))
      (switch string _returnvalue
        (:Symbol1
          (Utilities|Array|SetArrayElem (Variables|/Game/Bomb/BombController.BombController_C|GetSymbolLights _asbomb_controller_2) 0 false))
        (:Symbol2
          (Utilities|Array|SetArrayElem (Variables|/Game/Bomb/BombController.BombController_C|GetSymbolLights _asbomb_controller_2) 1 false))
        (:Symbol3
          (Utilities|Array|SetArrayElem (Variables|/Game/Bomb/BombController.BombController_C|GetSymbolLights _asbomb_controller_2) 2 false))
        (:Symbol4
          (Utilities|Array|SetArrayElem (Variables|/Game/Bomb/BombController.BombController_C|GetSymbolLights _asbomb_controller_2) 3 false))))))

(event OnClicked(StaticMesh1)
  (params (TouchedComponent :type Primitive%20Component%20Object%20Reference) (ButtonPressed :type Key%20Structure))
  (bind _returnvalue (Class|Actor|GetActorLabel))
  (bind _returnvalue_2 (Game|GetPlayerController 0))
  (bind _staticmeshcomponent (Variables|Debug|GetStaticMeshComponent))
  (if (Variables|Default|GetRed)
    (Rendering|Material|SetMaterial _staticmeshcomponent 0 "/Game/Bomb/BombParts/Materials/green_Mat.green_Mat")
    (Variables|Default|SetRed false)
    (bind _asbomb_controller (Utilities|Casting|CastToBombController _returnvalue_2))
    (switch string _returnvalue
      (:Symbol1
        (Utilities|Array|SetArrayElem (Variables|/Game/Bomb/BombController.BombController_C|GetSymbolLights _asbomb_controller) 0 true))
      (:Symbol2
        (Utilities|Array|SetArrayElem (Variables|/Game/Bomb/BombController.BombController_C|GetSymbolLights _asbomb_controller) 1 true))
      (:Symbol3
        (Utilities|Array|SetArrayElem (Variables|/Game/Bomb/BombController.BombController_C|GetSymbolLights _asbomb_controller) 2 true))
      (:Symbol4
        (Utilities|Array|SetArrayElem (Variables|/Game/Bomb/BombController.BombController_C|GetSymbolLights _asbomb_controller) 3 true)))
    (else
      (Rendering|Material|SetMaterial _staticmeshcomponent 0 "/Game/Bomb/BombParts/Materials/red_Mat.red_Mat")
      (Variables|Default|SetRed true)
      (bind _asbomb_controller_2 (Utilities|Casting|CastToBombController _returnvalue_2))
      (switch string _returnvalue
        (:Symbol1
          (Utilities|Array|SetArrayElem (Variables|/Game/Bomb/BombController.BombController_C|GetSymbolLights _asbomb_controller_2) 0 false))
        (:Symbol2
          (Utilities|Array|SetArrayElem (Variables|/Game/Bomb/BombController.BombController_C|GetSymbolLights _asbomb_controller_2) 1 false))
        (:Symbol3
          (Utilities|Array|SetArrayElem (Variables|/Game/Bomb/BombController.BombController_C|GetSymbolLights _asbomb_controller_2) 2 false))
        (:Symbol4
          (Utilities|Array|SetArrayElem (Variables|/Game/Bomb/BombController.BombController_C|GetSymbolLights _asbomb_controller_2) 3 false))))))

(event EventBeginPlay
  (Utilities|FlowControl|Delay 1.0)
  (bind _asbomb_controller (Utilities|Casting|CastToBombController (Game|GetPlayerController 0)))
  (switch string (Class|Actor|GetActorLabel)
    (:Symbol1
      (Variables|Default|SetRandom (Utilities|Array|Get(acopy) (Variables|/Game/Bomb/BombController.BombController_C|GetSymArray _asbomb_controller))))
    (:Symbol2
      (Variables|Default|SetRandom (Utilities|Array|Get(acopy) (Variables|/Game/Bomb/BombController.BombController_C|GetSymArray _asbomb_controller) 1)))
    (:Symbol3
      (Variables|Default|SetRandom (Utilities|Array|Get(acopy) (Variables|/Game/Bomb/BombController.BombController_C|GetSymArray _asbomb_controller) 2)))
    (:Symbol4
      (Variables|Default|SetRandom (Utilities|Array|Get(acopy) (Variables|/Game/Bomb/BombController.BombController_C|GetSymArray _asbomb_controller) 3))))
  (switch int (Variables|Default|GetRandom)
    (:0
      (Variables|Default|SetMaterial "/Game/Bomb/BombParts/Materials/1_Mat.1_Mat"))
    (:1
      (Variables|Default|SetMaterial "/Game/Bomb/BombParts/Materials/2_Mat.2_Mat"))
    (:2
      (Variables|Default|SetMaterial "/Game/Bomb/BombParts/Materials/3_Mat.3_Mat"))
    (:3
      (Variables|Default|SetMaterial "/Game/Bomb/BombParts/Materials/4_Mat.4_Mat"))
    (:4
      (Variables|Default|SetMaterial "/Game/Bomb/BombParts/Materials/5_Mat.5_Mat"))
    (:5
      (Variables|Default|SetMaterial "/Game/Bomb/BombParts/Materials/6_Mat.6_Mat"))
    (:6
      (Variables|Default|SetMaterial "/Game/Bomb/BombParts/Materials/7_Mat.7_Mat"))
    (:7
      (Variables|Default|SetMaterial "/Game/Bomb/BombParts/Materials/8_Mat.8_Mat"))
    (:8
      (Variables|Default|SetMaterial "/Game/Bomb/BombParts/Materials/9_Mat.9_Mat"))
    (:9
      (Variables|Default|SetMaterial "/Game/Bomb/BombParts/Materials/10_Mat.10_Mat"))
    (:10
      (Variables|Default|SetMaterial "/Game/Bomb/BombParts/Materials/11_Mat.11_Mat")))
  (Rendering|Material|SetMaterial (Variables|Default|GetStaticMesh1) 0 (Variables|Default|GetMaterial)))

(event EventTick
  (params (DeltaSeconds :type Float%20%28single-precision%29))
  (bind _returnvalue (Class|Actor|GetActorLabel))
  (bind _returnvalue_2 (Game|GetPlayerController 0))
  (bind _staticmeshcomponent (Variables|Debug|GetStaticMeshComponent))
  (bind _asmotion_controller_pawn (Utilities|Casting|CastToMotionControllerPawn (Game|Player|GetPlayerPawn 0)))
  (Utilities|Casting|CastToBombController (Game|GetPlayerController 0))
  (if (Utilities|Enum|Equal(Enum) (Variables|/Game/VirtualRealityBP/Blueprints/MotionControllerPawn.MotionControllerPawn_C|GetHit _asmotion_controller_pawn) (Class|Actor|GetActorLabel))
    (if (Variables|Default|GetRed)
      (Rendering|Material|SetMaterial _staticmeshcomponent 0 "/Game/Bomb/BombParts/Materials/green_Mat.green_Mat")
      (Variables|Default|SetRed false)
      (bind _asbomb_controller (Utilities|Casting|CastToBombController _returnvalue_2))
      (switch string _returnvalue
        (:Symbol1
          (Utilities|Array|SetArrayElem (Variables|/Game/Bomb/BombController.BombController_C|GetSymbolLights _asbomb_controller) 0 true))
        (:Symbol2
          (Utilities|Array|SetArrayElem (Variables|/Game/Bomb/BombController.BombController_C|GetSymbolLights _asbomb_controller) 1 true))
        (:Symbol3
          (Utilities|Array|SetArrayElem (Variables|/Game/Bomb/BombController.BombController_C|GetSymbolLights _asbomb_controller) 2 true))
        (:Symbol4
          (Utilities|Array|SetArrayElem (Variables|/Game/Bomb/BombController.BombController_C|GetSymbolLights _asbomb_controller) 3 true)))
      (else
        (Rendering|Material|SetMaterial _staticmeshcomponent 0 "/Game/Bomb/BombParts/Materials/red_Mat.red_Mat")
        (Variables|Default|SetRed true)
        (bind _asbomb_controller_2 (Utilities|Casting|CastToBombController _returnvalue_2))
        (switch string _returnvalue
          (:Symbol1
            (Utilities|Array|SetArrayElem (Variables|/Game/Bomb/BombController.BombController_C|GetSymbolLights _asbomb_controller_2) 0 false))
          (:Symbol2
            (Utilities|Array|SetArrayElem (Variables|/Game/Bomb/BombController.BombController_C|GetSymbolLights _asbomb_controller_2) 1 false))
          (:Symbol3
            (Utilities|Array|SetArrayElem (Variables|/Game/Bomb/BombController.BombController_C|GetSymbolLights _asbomb_controller_2) 2 false))
          (:Symbol4
            (Utilities|Array|SetArrayElem (Variables|/Game/Bomb/BombController.BombController_C|GetSymbolLights _asbomb_controller_2) 3 false)))))))

(fn ConstructionScript)