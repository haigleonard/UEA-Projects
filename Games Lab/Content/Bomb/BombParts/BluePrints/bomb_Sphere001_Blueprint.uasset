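; A clickable sphere part of the bomb, apparently the button for a "Bop It" style module, that shows module state through its material.
; Each Tick polls BombController, showing green when its Bop count equals 20, white while BopIt has entries or the local Bop flag is set, otherwise black.
; A mouse click, or the VR pawn's Hit matching this actor's label, clears BopIt and sets that flag, which is never reset here.
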(event OnClicked(StaticMeshComponent)
  (params (TouchedComponent :type Primitive%20Component%20Object%20Reference) (ButtonPressed :type Key%20Structure))
  (Utilities|Array|Clear (Variables|/Game/Bomb/BombController.BombController_C|GetBopIt (stale EventTick _asbomb_controller)))
  (Variables|Default|SetBop true))

(event EventTick
  (params (DeltaSeconds :type Float%20%28single-precision%29))
  (bind _returnvalue (Game|GetPlayerController 0))
  (Utilities|FlowControl|Sequence
    (:then_0
      (bind _asbomb_controller (Utilities|Casting|CastToBombController _returnvalue))
      (bind _asbomb_controller_2 (Utilities|Casting|CastToBombController _returnvalue))
      (if (== (Variables|/Game/Bomb/BombController.BombController_C|GetBop _asbomb_controller_2) 20)
        (Rendering|Material|SetMaterial (Variables|Debug|GetStaticMeshComponent) 0 "/Game/Bomb/BombParts/Materials/green_Mat.green_Mat")
        (elif (or (> (Utilities|Array|Length (Variables|/Game/Bomb/BombController.BombController_C|GetBopIt _asbomb_controller)) 0) (Variables|Default|GetBop))
          (Rendering|Material|SetMaterial (Variables|Debug|GetStaticMeshComponent) 0 "/Game/Bomb/BombParts/Materials/white_Mat.white_Mat")
          (else
            (Rendering|Material|SetMaterial (Variables|Debug|GetStaticMeshComponent) 0 "/Game/Bomb/BombParts/Materials/Black_Mat.Black_Mat")))))
    (:then_1
      (bind _asmotion_controller_pawn (Utilities|Casting|CastToMotionControllerPawn (Game|Player|GetPlayerPawn 0)))
      (Utilities|Casting|CastToBombController (Game|GetPlayerController 0))
      (if (Utilities|Enum|Equal(Enum) (Variables|/Game/VirtualRealityBP/Blueprints/MotionControllerPawn.MotionControllerPawn_C|GetHit _asmotion_controller_pawn) (Class|Actor|GetActorLabel))
        (Utilities|Array|Clear (Variables|/Game/Bomb/BombController.BombController_C|GetBopIt _asbomb_controller))
        (Variables|Default|SetBop true)))))

(fn ConstructionScript)