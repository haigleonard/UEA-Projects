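; A bomb keypad button for one digit, toggled between red and green by the player.
; Each instance identifies its digit by matching its actor label, which selects its number material on BeginPlay.
; Mouse clicks flip the state, as does every Tick where the MotionControllerPawn's Hit equals the label.
; Tick also writes the state into that digit's slot in BombController's KeyPad array, with green as true.
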(event OnClicked(StaticMesh)
  (params (TouchedComponent :type Primitive%20Component%20Object%20Reference) (ButtonPressed :type Key%20Structure))
  (bind _staticmesh1 (Variables|Default|GetStaticMesh1))
  (if (Variables|Default|GetRed)
    (Rendering|Material|SetMaterial _staticmesh1 0 "/Game/Bomb/BombParts/Materials/green_Mat.green_Mat")
    (Variables|Default|SetRed false)
    (else
      (Rendering|Material|SetMaterial _staticmesh1 0 "/Game/Bomb/BombParts/Materials/red_Mat.red_Mat")
      (Variables|Default|SetRed true))))

(event OnClicked(StaticMesh1)
  (params (TouchedComponent :type Primitive%20Component%20Object%20Reference) (ButtonPressed :type Key%20Structure))
  (bind _staticmesh1 (Variables|Default|GetStaticMesh1))
  (if (Variables|Default|GetRed)
    (Rendering|Material|SetMaterial _staticmesh1 0 "/Game/Bomb/BombParts/Materials/green_Mat.green_Mat")
    (Variables|Default|SetRed false)
    (else
      (Rendering|Material|SetMaterial _staticmesh1 0 "/Game/Bomb/BombParts/Materials/red_Mat.red_Mat")
      (Variables|Default|SetRed true))))

(event OnClicked(StaticMeshComponent)
  (params (TouchedComponent :type Primitive%20Component%20Object%20Reference) (ButtonPressed :type Key%20Structure))
  (bind _staticmesh1 (Variables|Default|GetStaticMesh1))
  (if (Variables|Default|GetRed)
    (Rendering|Material|SetMaterial _staticmesh1 0 "/Game/Bomb/BombParts/Materials/green_Mat.green_Mat")
    (Variables|Default|SetRed false)
    (else
      (Rendering|Material|SetMaterial _staticmesh1 0 "/Game/Bomb/BombParts/Materials/red_Mat.red_Mat")
      (Variables|Default|SetRed true))))

(event EventBeginPlay
  (switch string (Class|Actor|GetActorLabel)
    (:bomb_KeyPad_Blueprint0
      (Variables|Default|SetNumberMat "/Game/Bomb/BombParts/Materials/KeyPad/0_Mat.0_Mat"))
    (:bomb_KeyPad_Blueprint1
      (Variables|Default|SetNumberMat "/Game/Bomb/BombParts/Materials/KeyPad/1_Mat.1_Mat"))
    (:bomb_KeyPad_Blueprint2
      (Variables|Default|SetNumberMat "/Game/Bomb/BombParts/Materials/KeyPad/2_Mat.2_Mat"))
    (:bomb_KeyPad_Blueprint3
      (Variables|Default|SetNumberMat "/Game/Bomb/BombParts/Materials/KeyPad/3_Mat.3_Mat"))
    (:bomb_KeyPad_Blueprint4
      (Variables|Default|SetNumberMat "/Game/Bomb/BombParts/Materials/KeyPad/4_Mat.4_Mat"))
    (:bomb_KeyPad_Blueprint5
      (Variables|Default|SetNumberMat "/Game/Bomb/BombParts/Materials/KeyPad/5_Mat.5_Mat"))
    (:bomb_KeyPad_Blueprint6
      (Variables|Default|SetNumberMat "/Game/Bomb/BombParts/Materials/KeyPad/6_Mat.6_Mat"))
    (:bomb_KeyPad_Blueprint7
      (Variables|Default|SetNumberMat "/Game/Bomb/BombParts/Materials/KeyPad/7_Mat.7_Mat"))
    (:bomb_KeyPad_Blueprint8
      (Variables|Default|SetNumberMat "/Game/Bomb/BombParts/Materials/KeyPad/8_Mat.8_Mat"))
    (:bomb_KeyPad_Blueprint9
      (Variables|Default|SetNumberMat "/Game/Bomb/BombParts/Materials/KeyPad/9_Mat.9_Mat")))
  (Rendering|Material|SetMaterial (Variables|Default|GetStaticMesh) 0 (Variables|Default|GetNumberMat)))

(event Collision|EventActorBeginOverlap
  (params (OtherActor :type Actor%20Object%20Reference)))

(event EventTick
  (params (DeltaSeconds :type Float%20%28single-precision%29))
  (bind _returnvalue (Class|Actor|GetActorLabel))
  (bind _staticmesh1 (Variables|Default|GetStaticMesh1))
  (Utilities|FlowControl|Sequence
    (:then_0
      (bind _asbomb_controller (Utilities|Casting|CastToBombController (Game|GetPlayerController 0)))
      (if (Variables|Default|GetRed)
        (switch string _returnvalue
          (:bomb_KeyPad_Blueprint0
            (Utilities|Array|SetArrayElem (Variables|/Game/Bomb/BombController.BombController_C|GetKeyPad _asbomb_controller) 0 false))
          (:bomb_KeyPad_Blueprint1
            (Utilities|Array|SetArrayElem (Variables|/Game/Bomb/BombController.BombController_C|GetKeyPad _asbomb_controller) 1 false))
          (:bomb_KeyPad_Blueprint2
            (Utilities|Array|SetArrayElem (Variables|/Game/Bomb/BombController.BombController_C|GetKeyPad _asbomb_controller) 2 false))
          (:bomb_KeyPad_Blueprint3
            (Utilities|Array|SetArrayElem (Variables|/Game/Bomb/BombController.BombController_C|GetKeyPad _asbomb_controller) 3 false))
          (:bomb_KeyPad_Blueprint4
            (Utilities|Array|SetArrayElem (Variables|/Game/Bomb/BombController.BombController_C|GetKeyPad _asbomb_controller) 4 false))
          (:bomb_KeyPad_Blueprint5
            (Utilities|Array|SetArrayElem (Variables|/Game/Bomb/BombController.BombController_C|GetKeyPad _asbomb_controller) 5 false))
          (:bomb_KeyPad_Blueprint6
            (Utilities|Array|SetArrayElem (Variables|/Game/Bomb/BombController.BombController_C|GetKeyPad _asbomb_controller) 6 false))
          (:bomb_KeyPad_Blueprint7
            (Utilities|Array|SetArrayElem (Variables|/Game/Bomb/BombController.BombController_C|GetKeyPad _asbomb_controller) 7 false))
          (:bomb_KeyPad_Blueprint8
            (Utilities|Array|SetArrayElem (Variables|/Game/Bomb/BombController.BombController_C|GetKeyPad _asbomb_controller) 8 false))
          (:bomb_KeyPad_Blueprint9
            (Utilities|Array|SetArrayElem (Variables|/Game/Bomb/BombController.BombController_C|GetKeyPad _asbomb_controller) 9 false)))
        (else
          (switch string _returnvalue
            (:bomb_KeyPad_Blueprint0
              (Utilities|Array|SetArrayElem (Variables|/Game/Bomb/BombController.BombController_C|GetKeyPad _asbomb_controller) 0 true))
            (:bomb_KeyPad_Blueprint1
              (Utilities|Array|SetArrayElem (Variables|/Game/Bomb/BombController.BombController_C|GetKeyPad _asbomb_controller) 1 true))
            (:bomb_KeyPad_Blueprint2
              (Utilities|Array|SetArrayElem (Variables|/Game/Bomb/BombController.BombController_C|GetKeyPad _asbomb_controller) 2 true))
            (:bomb_KeyPad_Blueprint3
              (Utilities|Array|SetArrayElem (Variables|/Game/Bomb/BombController.BombController_C|GetKeyPad _asbomb_controller) 3 true))
            (:bomb_KeyPad_Blueprint4
              (Utilities|Array|SetArrayElem (Variables|/Game/Bomb/BombController.BombController_C|GetKeyPad _asbomb_controller) 4 true))
            (:bomb_KeyPad_Blueprint5
              (Utilities|Array|SetArrayElem (Variables|/Game/Bomb/BombController.BombController_C|GetKeyPad _asbomb_controller) 5 true))
            (:bomb_KeyPad_Blueprint6
              (Utilities|Array|SetArrayElem (Variables|/Game/Bomb/BombController.BombController_C|GetKeyPad _asbomb_controller) 6 true))
            (:bomb_KeyPad_Blueprint7
              (Utilities|Array|SetArrayElem (Variables|/Game/Bomb/BombController.BombController_C|GetKeyPad _asbomb_controller) 7 true))
            (:bomb_KeyPad_Blueprint8
              (Utilities|Array|SetArrayElem (Variables|/Game/Bomb/BombController.BombController_C|GetKeyPad _asbomb_controller) 8 true))
            (:bomb_KeyPad_Blueprint9
              (Utilities|Array|SetArrayElem (Variables|/Game/Bomb/BombController.BombController_C|GetKeyPad _asbomb_controller) 9 true))))))
    (:then_1
      (bind _asmotion_controller_pawn (Utilities|Casting|CastToMotionControllerPawn (Game|Player|GetPlayerPawn 0)))
      (Utilities|Casting|CastToBombController (Game|GetPlayerController 0))
      (if (Utilities|Enum|Equal(Enum) (Variables|/Game/VirtualRealityBP/Blueprints/MotionControllerPawn.MotionControllerPawn_C|GetHit _asmotion_controller_pawn) (Class|Actor|GetActorLabel))
        (if (Variables|Default|GetRed)
          (Rendering|Material|SetMaterial _staticmesh1 0 "/Game/Bomb/BombParts/Materials/green_Mat.green_Mat")
          (Variables|Default|SetRed false)
          (else
            (Rendering|Material|SetMaterial _staticmesh1 0 "/Game/Bomb/BombParts/Materials/red_Mat.red_Mat")
            (Variables|Default|SetRed true)))))))

(fn ConstructionScript)