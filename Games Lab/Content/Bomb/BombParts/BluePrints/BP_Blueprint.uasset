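; A bomb part actor that rotates in 45-degree pitch steps and records its angle in the BombController.
; Each Tick rotates it while the MotionControllerPawn's Hit value matches its actor label, and clicking its StaticMesh runs the same step directly.
; Each step turns the actor by negative 45 degrees locally and adds 45 to the controller's Degrees, resetting that count to zero at 360.
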(event OnClicked(StaticMesh)
  (params (TouchedComponent :type Primitive%20Component%20Object%20Reference) (ButtonPressed :type Key%20Structure))
  (bind _returnvalue (Game|GetPlayerController 0))
  (Transformation|AddActorLocalRotation (Math|Rotator|MakeRotator 0.0 -45.0 0.0) false false)
  (bind _asbomb_controller (Utilities|Casting|CastToBombController _returnvalue))
  (Variables|/Game/Bomb/BombController.BombController_C|SetDegrees _asbomb_controller (+ (Variables|/Game/Bomb/BombController.BombController_C|GetDegrees _asbomb_controller) 45))
  (if (== (Variables|/Game/Bomb/BombController.BombController_C|GetDegrees _asbomb_controller) 360)
    (bind _asbomb_controller_2 (Utilities|Casting|CastToBombController _returnvalue))
    (Variables|/Game/Bomb/BombController.BombController_C|SetDegrees _asbomb_controller_2 0)))

(event EventTick
  (params (DeltaSeconds :type Float%20%28single-precision%29))
  (bind _returnvalue (Game|GetPlayerController 0))
  (bind _asmotion_controller_pawn (Utilities|Casting|CastToMotionControllerPawn (Game|Player|GetPlayerPawn 0)))
  (Utilities|Casting|CastToBombController (Game|GetPlayerController 0))
  (if (Utilities|Enum|Equal(Enum) (Variables|/Game/VirtualRealityBP/Blueprints/MotionControllerPawn.MotionControllerPawn_C|GetHit _asmotion_controller_pawn) (Class|Actor|GetActorLabel))
    (Transformation|AddActorLocalRotation (Math|Rotator|MakeRotator 0.0 -45.0 0.0) false false)
    (bind _asbomb_controller (Utilities|Casting|CastToBombController _returnvalue))
    (Variables|/Game/Bomb/BombController.BombController_C|SetDegrees _asbomb_controller (+ (Variables|/Game/Bomb/BombController.BombController_C|GetDegrees _asbomb_controller) 45))
    (if (== (Variables|/Game/Bomb/BombController.BombController_C|GetDegrees _asbomb_controller) 360)
      (bind _asbomb_controller_2 (Utilities|Casting|CastToBombController _returnvalue))
      (Variables|/Game/Bomb/BombController.BombController_C|SetDegrees _asbomb_controller_2 0))))

(fn ConstructionScript)