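; Clickable wire on a bomb puzzle that takes a random red, blue, green or yellow material at BeginPlay.
; It records the color index in the BombController's Wires and WireSol arrays, choosing its slot among five by hard-coded actor label.
; A click, or a Tick check matching MotionControllerPawn's Hit to its label, swaps in a second mesh of the same color and marks only the Wires slot as 4.
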(event OnClicked(Box)
  (params (TouchedComponent :type Primitive%20Component%20Object%20Reference) (ButtonPressed :type Key%20Structure))
  (Rendering|SetVisibility (Variables|Debug|GetStaticMeshComponent) false false)
  (Rendering|SetVisibility (Variables|Default|GetStaticMesh) true false)
  (Rendering|Material|SetMaterial (Variables|Default|GetStaticMesh) 0 (Variables|Default|GetMaterial))
  (bind _asbomb_controller (Utilities|Casting|CastToBombController (Game|GetPlayerController 0)))
  (switch string (Class|Actor|GetActorLabel)
    (:bomb_WireR_Blueprint1
      (Utilities|Array|SetArrayElem (Variables|/Game/Bomb/BombController.BombController_C|GetWires _asbomb_controller) 0 4))
    (:bomb_WireR_Blueprint2
      (Utilities|Array|SetArrayElem (Variables|/Game/Bomb/BombController.BombController_C|GetWires _asbomb_controller) 1 4))
    (:bomb_WireR_Blueprint3
      (Utilities|Array|SetArrayElem (Variables|/Game/Bomb/BombController.BombController_C|GetWires _asbomb_controller) 2 4))
    (:bomb_WireR_Blueprint4
      (Utilities|Array|SetArrayElem (Variables|/Game/Bomb/BombController.BombController_C|GetWires _asbomb_controller) 3 4))
    (:bomb_WireR_Blueprint5
      (Utilities|Array|SetArrayElem (Variables|/Game/Bomb/BombController.BombController_C|GetWires _asbomb_controller) 4 4))))

(event EventBeginPlay
  (bind _output_get (Variables|Default|SetRandom (Math|Random|RandomInteger 4)))
  (switch int _output_get
    (:0
      (Variables|Default|SetMaterial "/Game/Bomb/BombParts/Materials/red_Mat.red_Mat"))
    (:1
      (Variables|Default|SetMaterial "/Game/Bomb/BombParts/Materials/Blue_Mat.Blue_Mat"))
    (:2
      (Variables|Default|SetMaterial "/Game/Bomb/BombParts/Materials/green_Mat.green_Mat"))
    (:3
      (Variables|Default|SetMaterial "/Game/Bomb/BombParts/Materials/yellow_Mat.yellow_Mat")))
  (Rendering|Material|SetMaterial (Variables|Debug|GetStaticMeshComponent) 0 (Variables|Default|GetMaterial))
  (bind _asbomb_controller (Utilities|Casting|CastToBombController (Game|GetPlayerController 0)))
  (switch string (Class|Actor|GetActorLabel)
    (:bomb_WireR_Blueprint1
      (Utilities|Array|SetArrayElem (Variables|/Game/Bomb/BombController.BombController_C|GetWires _asbomb_controller) 0 (Variables|Default|GetRandom))
      (Utilities|Array|SetArrayElem (Variables|/Game/Bomb/BombController.BombController_C|GetWireSol _asbomb_controller) 0 (Variables|Default|GetRandom)))
    (:bomb_WireR_Blueprint2
      (Utilities|Array|SetArrayElem (Variables|/Game/Bomb/BombController.BombController_C|GetWires _asbomb_controller) 1 (Variables|Default|GetRandom))
      (Utilities|Array|SetArrayElem (Variables|/Game/Bomb/BombController.BombController_C|GetWireSol _asbomb_controller) 1 (Variables|Default|GetRandom)))
    (:bomb_WireR_Blueprint3
      (Utilities|Array|SetArrayElem (Variables|/Game/Bomb/BombController.BombController_C|GetWires _asbomb_controller) 2 (Variables|Default|GetRandom))
      (Utilities|Array|SetArrayElem (Variables|/Game/Bomb/BombController.BombController_C|GetWireSol _asbomb_controller) 2 (Variables|Default|GetRandom)))
    (:bomb_WireR_Blueprint4
      (Utilities|Array|SetArrayElem (Variables|/Game/Bomb/BombController.BombController_C|GetWires _asbomb_controller) 3 (Variables|Default|GetRandom))
      (Utilities|Array|SetArrayElem (Variables|/Game/Bomb/BombController.BombController_C|GetWireSol _asbomb_controller) 3 (Variables|Default|GetRandom)))
    (:bomb_WireR_Blueprint5
      (Utilities|Array|SetArrayElem (Variables|/Game/Bomb/BombController.BombController_C|GetWires _asbomb_controller) 4 (Variables|Default|GetRandom))
      (Utilities|Array|SetArrayElem (Variables|/Game/Bomb/BombController.BombController_C|GetWireSol _asbomb_controller) 4 (Variables|Default|GetRandom)))))

(event Collision|EventActorBeginOverlap
  (params (OtherActor :type Actor%20Object%20Reference)))

(event EventTick
  (params (DeltaSeconds :type Float%20%28single-precision%29))
  (bind _asmotion_controller_pawn (Utilities|Casting|CastToMotionControllerPawn (Game|Player|GetPlayerPawn 0)))
  (Utilities|Casting|CastToBombController (Game|GetPlayerController 0))
  (if (Utilities|Enum|Equal(Enum) (Variables|/Game/VirtualRealityBP/Blueprints/MotionControllerPawn.MotionControllerPawn_C|GetHit _asmotion_controller_pawn) (Class|Actor|GetActorLabel))
    (Rendering|SetVisibility (Variables|Debug|GetStaticMeshComponent) false false)
    (Rendering|SetVisibility (Variables|Default|GetStaticMesh) true false)
    (Rendering|Material|SetMaterial (Variables|Default|GetStaticMesh) 0 (Variables|Default|GetMaterial))
    (bind _asbomb_controller (Utilities|Casting|CastToBombController (Game|GetPlayerController 0)))
    (switch string (Class|Actor|GetActorLabel)
      (:bomb_WireR_Blueprint1
        (Utilities|Array|SetArrayElem (Variables|/Game/Bomb/BombController.BombController_C|GetWires _asbomb_controller) 0 4))
      (:bomb_WireR_Blueprint2
        (Utilities|Array|SetArrayElem (Variables|/Game/Bomb/BombController.BombController_C|GetWires _asbomb_controller) 1 4))
      (:bomb_WireR_Blueprint3
        (Utilities|Array|SetArrayElem (Variables|/Game/Bomb/BombController.BombController_C|GetWires _asbomb_controller) 2 4))
      (:bomb_WireR_Blueprint4
        (Utilities|Array|SetArrayElem (Variables|/Game/Bomb/BombController.BombController_C|GetWires _asbomb_controller) 3 4))
      (:bomb_WireR_Blueprint5
        (Utilities|Array|SetArrayElem (Variables|/Game/Bomb/BombController.BombController_C|GetWires _asbomb_controller) 4 4)))))

(fn ConstructionScript)