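; Bomb part plane that shows a random digit and contributes it to the bomb's solution code.
; On BeginPlay it rolls 0 to 9 and applies the matching number material to its mesh.
; It then uses its actor label (Plane 2 Blueprint 1 to 6) as a decimal place and adds the weighted digit to KSol on the BombController player controller, so six instances form a six-digit value.
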(event EventBeginPlay
  (bind _output_get (Variables|Default|SetRandom (Math|Random|RandomInteger 10)))
  (switch int _output_get
    (:0
      (Variables|Default|SetNumberMat "/Game/Bomb/BombParts/Materials/KeyPad/0_Mat.0_Mat"))
    (:1
      (Variables|Default|SetNumberMat "/Game/Bomb/BombParts/Materials/KeyPad/1_Mat.1_Mat"))
    (:2
      (Variables|Default|SetNumberMat "/Game/Bomb/BombParts/Materials/KeyPad/2_Mat.2_Mat"))
    (:3
      (Variables|Default|SetNumberMat "/Game/Bomb/BombParts/Materials/KeyPad/3_Mat.3_Mat"))
    (:4
      (Variables|Default|SetNumberMat "/Game/Bomb/BombParts/Materials/KeyPad/4_Mat.4_Mat"))
    (:5
      (Variables|Default|SetNumberMat "/Game/Bomb/BombParts/Materials/KeyPad/5_Mat.5_Mat"))
    (:6
      (Variables|Default|SetNumberMat "/Game/Bomb/BombParts/Materials/KeyPad/6_Mat.6_Mat"))
    (:7
      (Variables|Default|SetNumberMat "/Game/Bomb/BombParts/Materials/KeyPad/7_Mat.7_Mat"))
    (:8
      (Variables|Default|SetNumberMat "/Game/Bomb/BombParts/Materials/KeyPad/8_Mat.8_Mat"))
    (:9
      (Variables|Default|SetNumberMat "/Game/Bomb/BombParts/Materials/KeyPad/9_Mat.9_Mat")))
  (Rendering|Material|SetMaterial (Variables|Debug|GetStaticMeshComponent) 0 (Variables|Default|GetNumberMat))
  (bind _asbomb_controller (Utilities|Casting|CastToBombController (Game|GetPlayerController 0)))
  (switch string (Class|Actor|GetActorLabel)
    (:Plane2_Blueprint1
      (Variables|/Game/Bomb/BombController.BombController_C|SetKSol _asbomb_controller (+ (* (Variables|Default|GetRandom) 100000) (Variables|/Game/Bomb/BombController.BombController_C|GetKSol _asbomb_controller))))
    (:Plane2_Blueprint2
      (Variables|/Game/Bomb/BombController.BombController_C|SetKSol _asbomb_controller (+ (* (Variables|Default|GetRandom) 10000) (Variables|/Game/Bomb/BombController.BombController_C|GetKSol _asbomb_controller))))
    (:Plane2_Blueprint3
      (Variables|/Game/Bomb/BombController.BombController_C|SetKSol _asbomb_controller (+ (* (Variables|Default|GetRandom) 1000) (Variables|/Game/Bomb/BombController.BombController_C|GetKSol _asbomb_controller))))
    (:Plane2_Blueprint4
      (Variables|/Game/Bomb/BombController.BombController_C|SetKSol _asbomb_controller (+ (* (Variables|Default|GetRandom) 100) (Variables|/Game/Bomb/BombController.BombController_C|GetKSol _asbomb_controller))))
    (:Plane2_Blueprint5
      (Variables|/Game/Bomb/BombController.BombController_C|SetKSol _asbomb_controller (+ (* (Variables|Default|GetRandom) 10) (Variables|/Game/Bomb/BombController.BombController_C|GetKSol _asbomb_controller))))
    (:Plane2_Blueprint6
      (Variables|/Game/Bomb/BombController.BombController_C|SetKSol _asbomb_controller (+ (Variables|Default|GetRandom) (Variables|/Game/Bomb/BombController.BombController_C|GetKSol _asbomb_controller))))))

(event Collision|EventActorBeginOverlap
  (params (OtherActor :type Actor%20Object%20Reference)))

(event EventTick
  (params (DeltaSeconds :type Float%20%28single-precision%29)))

(fn ConstructionScript)