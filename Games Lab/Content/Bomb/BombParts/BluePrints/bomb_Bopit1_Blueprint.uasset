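; One of four colored Bop It buttons on the bomb, each identified by its actor label, that plays back a sequence and records player input.
; A click, or a motion controller pawn Hit matching the label on Tick, appends the button's number to BombController's BopIt array.
; While the bomb sphere's Bop flag is set, each button steps through BopItSol by tick count, flashing white on its turn, then clears the flag.
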(event OnClicked(StaticMeshComponent)
  (params (TouchedComponent :type Primitive%20Component%20Object%20Reference) (ButtonPressed :type Key%20Structure))
  (bind _asbomb_controller (Utilities|Casting|CastToBombController (Game|GetPlayerController 0)))
  (switch string (Class|Actor|GetActorLabel)
    (:bomb_Bopit1_Blueprint1
      (Utilities|Array|Add (Variables|/Game/Bomb/BombController.BombController_C|GetBopIt _asbomb_controller) 0))
    (:bomb_Bopit1_Blueprint2
      (Utilities|Array|Add (Variables|/Game/Bomb/BombController.BombController_C|GetBopIt _asbomb_controller) 1))
    (:bomb_Bopit1_Blueprint3
      (Utilities|Array|Add (Variables|/Game/Bomb/BombController.BombController_C|GetBopIt _asbomb_controller) 2))
    (:bomb_Bopit1_Blueprint4
      (Utilities|Array|Add (Variables|/Game/Bomb/BombController.BombController_C|GetBopIt _asbomb_controller) 3))))

(event EventBeginPlay)

(event Collision|EventActorBeginOverlap
  (params (OtherActor :type Actor%20Object%20Reference)))

(event EventTick
  (params (DeltaSeconds :type Float%20%28single-precision%29))
  (bind _returnvalue (Class|Actor|GetActorLabel))
  (Utilities|FlowControl|Sequence
    (:then_0
      (bind _asmotion_controller_pawn (Utilities|Casting|CastToMotionControllerPawn (Game|Player|GetPlayerPawn 0)))
      (bind _asbomb_controller (Utilities|Casting|CastToBombController (Game|GetPlayerController 0)))
      (if (Utilities|Enum|Equal(Enum) (Variables|/Game/VirtualRealityBP/Blueprints/MotionControllerPawn.MotionControllerPawn_C|GetHit _asmotion_controller_pawn) _returnvalue)
        (switch string _returnvalue
          (:bomb_Bopit1_Blueprint1
            (Utilities|Array|Add (Variables|/Game/Bomb/BombController.BombController_C|GetBopIt _asbomb_controller) 0))
          (:bomb_Bopit1_Blueprint2
            (Utilities|Array|Add (Variables|/Game/Bomb/BombController.BombController_C|GetBopIt _asbomb_controller) 1))
          (:bomb_Bopit1_Blueprint3
            (Utilities|Array|Add (Variables|/Game/Bomb/BombController.BombController_C|GetBopIt _asbomb_controller) 2))
          (:bomb_Bopit1_Blueprint4
            (Utilities|Array|Add (Variables|/Game/Bomb/BombController.BombController_C|GetBopIt _asbomb_controller) 3)))))
    (:then_1
      (bind _outactors (Actor|GetAllActorsOfClass "/Game/Bomb/BombParts/BluePrints/bomb_Sphere001_Blueprint.bomb_Sphere001_Blueprint_C"))
      (bind _asbomb_sphere_001_blueprint (Utilities|Casting|CastTobomb_Sphere001_Blueprint (Utilities|Array|Get(acopy) _outactors)))
      (if (Variables|/Game/Bomb/BombParts/BluePrints/bomb_Sphere001_Blueprint.bomb_Sphere001_Blueprint_C|GetBop _asbomb_sphere_001_blueprint)
        (bind _asbomb_controller_2 (Utilities|Casting|CastToBombController (Game|GetPlayerController 0)))
        (switch int (Utilities|Array|Get(acopy) (Variables|/Game/Bomb/BombController.BombController_C|GetBopItSol _asbomb_controller_2) (Variables|Default|Getindex))
          (:0
            (if (Utilities|Enum|Equal(Enum) (Class|Actor|GetActorLabel) "bomb_Bopit1_Blueprint1")
              (Rendering|Material|SetMaterial (Variables|Debug|GetStaticMeshComponent) 0 "/Game/Bomb/BombParts/Materials/white_Mat.white_Mat")
              (if (>= (Variables|Default|Gettimer) 50)
                (Rendering|Material|SetMaterial (Variables|Debug|GetStaticMeshComponent) 0 "/Game/Bomb/BombParts/Materials/red_Mat.red_Mat")
                (Variables|Default|Settimer 0 :!label _label)
                (bind _result (Math|Integer|IncrementInt (Variables|Default|Getindex))
                  (:%20%20
                    (Variables|Default|Setindex _result)
                    (if (>= (Variables|Default|Getindex) 21)
                      (Variables|Default|Setindex 0)
                      (bind _outactors_2 (Actor|GetAllActorsOfClass "/Game/Bomb/BombParts/BluePrints/bomb_Sphere001_Blueprint.bomb_Sphere001_Blueprint_C"))
                      (bind _asbomb_sphere_001_blueprint_2 (Utilities|Casting|CastTobomb_Sphere001_Blueprint (Utilities|Array|Get(acopy) _outactors_2)))
                      (Variables|/Game/Bomb/BombParts/BluePrints/bomb_Sphere001_Blueprint.bomb_Sphere001_Blueprint_C|SetBop _asbomb_sphere_001_blueprint_2 false)
                      (switch string (Class|Actor|GetActorLabel)
                        (:bomb_Bopit1_Blueprint1
                          (Rendering|Material|SetMaterial (Variables|Debug|GetStaticMeshComponent) 0 "/Game/Bomb/BombParts/Materials/red_Mat.red_Mat"))
                        (:bomb_Bopit1_Blueprint2
                          (Rendering|Material|SetMaterial (Variables|Debug|GetStaticMeshComponent) 0 "/Game/Bomb/BombParts/Materials/Blue_Mat.Blue_Mat"))
                        (:bomb_Bopit1_Blueprint3
                          (Rendering|Material|SetMaterial (Variables|Debug|GetStaticMeshComponent) 0 "/Game/Bomb/BombParts/Materials/green_Mat.green_Mat"))
                        (:bomb_Bopit1_Blueprint4
                          (Rendering|Material|SetMaterial (Variables|Debug|GetStaticMeshComponent) 0 "/Game/Geometry/Wires/Textures/yellow_Mat.yellow_Mat"))))))
                (else
                  (bind _result_2 (Math|Integer|IncrementInt (Variables|Default|Gettimer) :!label _label_2)
                    (:%20%20
                      (Variables|Default|Settimer _result_2)
                      (if (>= (Variables|Default|Gettimer) 51)
                        (goto _label))))))
              (else
                (goto _label_2))))
          (:1
            (if (Utilities|Enum|Equal(Enum) (Class|Actor|GetActorLabel) "bomb_Bopit1_Blueprint2")
              (Rendering|Material|SetMaterial (Variables|Debug|GetStaticMeshComponent) 0 "/Game/Bomb/BombParts/Materials/white_Mat.white_Mat")
              (if (>= (Variables|Default|Gettimer) 50)
                (Rendering|Material|SetMaterial (Variables|Debug|GetStaticMeshComponent) 0 "/Game/Bomb/BombParts/Materials/Blue_Mat.Blue_Mat")
                (goto _label)
                (else
                  (goto _label_2)))
              (else
                (goto _label_2))))
          (:2
            (if (Utilities|Enum|Equal(Enum) (Class|Actor|GetActorLabel) "bomb_Bopit1_Blueprint3")
              (Rendering|Material|SetMaterial (Variables|Debug|GetStaticMeshComponent) 0 "/Game/Bomb/BombParts/Materials/white_Mat.white_Mat")
              (if (>= (Variables|Default|Gettimer) 50)
                (Rendering|Material|SetMaterial (Variables|Debug|GetStaticMeshComponent) 0 "/Game/Bomb/BombParts/Materials/green_Mat.green_Mat")
                (goto _label)
                (else
                  (goto _label_2)))
              (else
                (goto _label_2))))
          (:3
            (if (Utilities|Enum|Equal(Enum) (Class|Actor|GetActorLabel) "bomb_Bopit1_Blueprint4")
              (Rendering|Material|SetMaterial (Variables|Debug|GetStaticMeshComponent) 0 "/Game/Bomb/BombParts/Materials/white_Mat.white_Mat")
              (if (>= (Variables|Default|Gettimer) 50)
                (Rendering|Material|SetMaterial (Variables|Debug|GetStaticMeshComponent) 0 "/Game/Geometry/Wires/Textures/yellow_Mat.yellow_Mat")
                (goto _label)
                (else
                  (goto _label_2)))
              (else
                (goto _label_2)))))))))

(fn ConstructionScript)