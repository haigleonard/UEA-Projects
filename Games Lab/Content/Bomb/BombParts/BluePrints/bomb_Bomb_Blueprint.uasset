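; Bomb actor that picks its random color and computes the degrees solution for a bomb puzzle on BeginPlay.
; After a short delay, a random index sets one of four mesh materials and adds a 90-degree step per index to 45 times each BombController Wires value.
; The sum is stored in the controller's DegreesSol and reduced by full turns, except the 720–1080 range, which becomes a constant -720.
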(event EventBeginPlay
  (Utilities|FlowControl|Delay 0.2)
  (bind _output_get (Variables|Default|SetRandom (Math|Random|RandomInteger 4)))
  (switch int _output_get
    (:0
      (Variables|Default|SetMaterial "/Game/Geometry/Wires/Textures/red_Mat.red_Mat"))
    (:1
      (Variables|Default|SetMaterial "/Game/Bomb/BombParts/Materials/Blue_Mat.Blue_Mat"))
    (:2
      (Variables|Default|SetMaterial "/Game/Bomb/BombParts/Materials/green_Mat.green_Mat"))
    (:3
      (Variables|Default|SetMaterial "/Game/Geometry/Wires/Textures/yellow_Mat.yellow_Mat")))
  (Rendering|Material|SetMaterial (Variables|Debug|GetStaticMeshComponent) 0 (Variables|Default|GetMaterial))
  (bind _asbomb_controller (Utilities|Casting|CastToBombController (Game|GetPlayerController 0)))
  (for _array_element (Variables|/Game/Bomb/BombController.BombController_C|GetWires _asbomb_controller)
    (Variables|Default|SetTotal (+ (* _array_element 45) (Variables|Default|GetTotal))))
  (bind _output_get_2 (Variables|/Game/Bomb/BombController.BombController_C|SetDegreesSol _asbomb_controller (+ (* (Variables|Default|GetRandom) 90) (Variables|Default|GetTotal))))
  (if (not (< _output_get_2 360))
    (if (and (>= _output_get_2 360) (< _output_get_2 720))
      (Variables|/Game/Bomb/BombController.BombController_C|SetDegreesSol _asbomb_controller (- _output_get_2 360))
      (elif (and (>= _output_get_2 720) (< _output_get_2 1080))
        (Variables|/Game/Bomb/BombController.BombController_C|SetDegreesSol _asbomb_controller (- 0 720))
        (else
          (Variables|/Game/Bomb/BombController.BombController_C|SetDegreesSol _asbomb_controller (- _output_get_2 1080)))))))

(fn ConstructionScript)