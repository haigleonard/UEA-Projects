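; Security camera Blueprint with a tinted spotlight, a CameraAI_BP controller and side colliders that reverse its sweep on hitting InstancedFloorActor geometry.
; UpdateCCTV refreshes light color and eye position; on authority, it yaws toward player 0 once sensed long enough, reverting if either collider overlaps geometry.
; GetClosestGuard returns the nearest ThirdPersonCharacter on a given floor by 2D distance.
; Remote instances give the camera mesh a different collision object type.
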(event Custom|OnComponentBeginOverlap_Event_0
  (params (OverlappedComponent :type Primitive%20Component%20Object%20Reference) (OtherActor :type Actor%20Object%20Reference) (OtherComp :type Primitive%20Component%20Object%20Reference) (OtherBodyIndex :type Integer) (bFromSweep :type Boolean) (SweepResult :type Hit%20Result%20Structure%20%28by%20ref%29))
  (Utilities|Casting|CastToInstancedFloorActor OtherActor)
  (Class|CCTVPawn|ChangeDirection))

(event EventBeginPlay
  (Networking|SwitchHasAuthority
    (:Authority
      _)
    (:Remote
      (Collision|SetCollisionObjectType (Variables|Default|GetCCTV_SM) "ECC_GameTraceChannel2")))
  (Collision|AssignOnComponentBeginOverlap (Variables|Default|GetLeftCollision) (delegate Custom|OnComponentBeginOverlap_Event_0))
  (Collision|AssignOnComponentBeginOverlap (Variables|Default|GetRightCollision) (delegate Custom|OnComponentBeginOverlap_Event_0))
  (Class|CCTVPawn|SetEyePosition (Transformation|GetWorldLocation (Variables|Default|GetEyeCentre))))

(event Collision|EventActorBeginOverlap
  (params (OtherActor :type Actor%20Object%20Reference)))

(event EventUpdateCCTV
  (bind _returnvalue (Transformation|GetActorRotation))
  (bind (_roll _pitch) (Math|Rotator|BreakRotator _returnvalue))
  (|CallParentFunction)
  (Rendering|Components|Light|SetLightColor (Variables|Default|GetSpotLight) (Math|Color|MakeColor (Variables|Default|GetlightRed) (Variables|Default|GetlightGreen) 0.0) true)
  (Class|CCTVPawn|SetEyePosition (Transformation|GetWorldLocation (Variables|Default|GetEyeCentre)))
  (bind _ascamera_ai_bp (Utilities|Casting|CastToCameraAI_BP (Pawn|GetController)))
  (bind _output_get (Variables|Default|SetsTime (Variables|/Game/Geometry/CCTV/CameraAI_BP.CameraAI_BP_C|GetsensedTime _ascamera_ai_bp)))
  (Networking|SwitchHasAuthority
    (:Authority
      (if (and (Variables|/Script/PCGTesting.CameraAIController|GetseesPlayer _ascamera_ai_bp) (> _output_get 1.5))
        (Variables|Default|SetoldRot (Transformation|GetActorRotation))
        (Transformation|SetActorRotation (Math|Rotator|MakeRotator _roll _pitch (.Yaw (Math|Rotator|BreakRotator (Math|Rotator|MakeRotfromX (- (Transformation|GetWorldLocation (Variables|/Script/Engine.Character|GetMesh (Game|GetPlayerCharacter 0))) (Transformation|GetActorLocation)))))))
        (if (not (and (== (Utilities|Array|Length (Collision|GetOverlappingActors (Variables|Default|GetRightCollision) "/Script/PCGTesting.InstancedFloorActor" :!class /Script/Engine.PrimitiveComponent)) 0) (== (Utilities|Array|Length (Collision|GetOverlappingActors (Variables|Default|GetLeftCollision) "/Script/PCGTesting.InstancedFloorActor" :!class /Script/Engine.PrimitiveComponent)) 0)))
          (Transformation|SetActorRotation (Variables|Default|GetoldRot)))))))

(event EventTick
  (params (DeltaSeconds :type Float%20%28single-precision%29)))

(fn ConstructionScript)

(fn GetClosestGuard
  (params (cameraLevel :type Integer))
  (bind _returnvalue (Transformation|GetActorLocation))
  (bind (_x _y) (Math|Vector|BreakVector _returnvalue))
  (bind _outactors (Actor|GetAllActorsOfClass "/Game/ThirdPersonCPP/Blueprints/ThirdPersonCharacter.ThirdPersonCharacter_C"))
  (for _array_element _outactors
    (if (== (Variables|/Script/PCGTesting.TP_ThirdPersonCharacter|Getfloor _array_element) cameraLevel)
      (if (<= (Variables|Default|GetclosestDist) 0.0)
        (Variables|Default|SetclosestDist (Math|Vector2D|Vector2DLength (- (Math|Vector2D|MakeVector2D (.X (Math|Vector|BreakVector (Transformation|GetActorLocation _array_element))) (.Y (Math|Vector|BreakVector (Transformation|GetActorLocation _array_element)))) (Math|Vector2D|MakeVector2D _x _y))) :!label _label)
        (Variables|Default|SetclosestGuard _array_element)
        (elif (< (Math|Vector2D|Vector2DLength (- (Math|Vector2D|MakeVector2D (.X (Math|Vector|BreakVector (Transformation|GetActorLocation _array_element))) (.Y (Math|Vector|BreakVector (Transformation|GetActorLocation _array_element)))) (Math|Vector2D|MakeVector2D _x _y))) (Variables|Default|GetclosestDist))
          (goto _label)))))
  (return (Variables|Default|GetclosestGuard)))