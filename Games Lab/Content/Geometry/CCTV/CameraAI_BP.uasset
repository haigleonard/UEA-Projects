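; CCTV camera AI Blueprint that tracks how long it has sensed the first player.
; On authority, Tick polls AIPerception for that player, setting SeesPlayer and raising SensedTime while seen or decaying it while unseen.
; The zero floor and upper cap apply only on the decay branch, so the timer grows unbounded while seen.
; GetSensedTime exposes the timer; OnPerceptionUpdated is empty and its debug printing is disconnected.
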(event OnPerceptionUpdated(AIPerception)
  (params (UpdatedActors :type Array%20of%20Actor%20Object%20References)))

(event EventBeginPlay)

(event EventTick
  (params (DeltaSeconds :type Float%20%28single-precision%29))
  (Networking|SwitchHasAuthority
    (:Authority
      (bind (_info _returnvalue) (Class|AIPerceptionComponent|GetActorsPerception (Variables|Default|GetAIPerception) (Game|Player|GetPlayerPawn 0)))
      (if _returnvalue
        (if (.bSuccessfullySensed (Utilities|Struct|BreakAIStimulus (Utilities|Array|Get(acopy) (.LastSensedStimuli (Utilities|Struct|BreakActorPerceptionBlueprintInfo _info)))))
          (Variables|Default|SetseesPlayer true)
          (Variables|Default|SetsensedTime (+ DeltaSeconds (Variables|Default|GetsensedTime)))
          (else
            (Variables|Default|SetseesPlayer false)
            (bind _output_get (Variables|Default|SetsensedTime (- (Variables|Default|GetsensedTime) DeltaSeconds)))
            (if (< _output_get 0.0)
              (Variables|Default|SetsensedTime 0.0)
              (elif (> _output_get 15.0)
                (Variables|Default|SetsensedTime 15.0)))))))))

(fn ConstructionScript)

(fn GetSensedTime
  (return (Variables|Default|GetsensedTime)))