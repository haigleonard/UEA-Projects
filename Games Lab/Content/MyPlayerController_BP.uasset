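; Player controller whose non-authority side lets a player click rooms to view through their hacked CCTV cameras.
; Left click traces for a room trigger, then the game mode's level actor supplies that room's camera for player controller 1 to possess if hacked.
; The next click returns that controller to the first IntelPawn.
; Each client tick also traces upward from player one's position to punch fog holes in masking actors.
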(event Custom|PossessCameraInroom
  (params (roomNum :type Integer) (floorNum :type Integer))
  (bind _asmy_tp_third_person_game_mode (Utilities|Casting|CastToMyTP_ThirdPersonGameMode (Game|GetGameMode)))
  (bind _returnvalue (Class|LevelActor|GetCCTVfromRoom (Variables|/Game/HUD/MyTP_ThirdPersonGameMode.MyTP_ThirdPersonGameMode_C|GetLevelActor _asmy_tp_third_person_game_mode) roomNum floorNum))
  (Utilities|IsValid _returnvalue
    (:Is%20Valid
      (bind _returnvalue_2 (Class|CCTVPawn|HackedCheck _returnvalue))
      (if _returnvalue_2
        (bind _asmy_player_controller_bp (Utilities|Casting|CastToMyPlayerController_BP (Game|GetPlayerController 1)))
        (Pawn|Possess _asmy_player_controller_bp _returnvalue)))))

(event Custom|ReleaseCamera
  (bind _asmy_player_controller_bp (Utilities|Casting|CastToMyPlayerController_BP (Game|GetPlayerController 1)))
  (bind _outactors (Actor|GetAllActorsOfClass "/Game/IntelPlayer/IntelPawn_BP.IntelPawn_BP_C"))
  (for (_array_element _array_index) _outactors
    (if (== _array_index 0)
      (Pawn|Possess _asmy_player_controller_bp _array_element))))

(event EventBeginPlay
  (Networking|SwitchHasAuthority
    (:Remote
      (Variables|Default|SetbShowMouseCursor true))))

(event EventTick
  (params (DeltaSeconds :type Float%20%28single-precision%29))
  (Networking|SwitchHasAuthority
    (:Remote
      (bind _asmy_game_state_base (Utilities|Casting|CastToMyGameStateBase (Game|GetGameState)))
      (bind _returnvalue (Class|MyGameStateBase|GetP1Location _asmy_game_state_base))
      (bind _returnvalue_2 (Class|MyGameStateBase|GetP1UpVector _asmy_game_state_base))
      (bind (_outhit _returnvalue_3) (Collision|LineTraceForObjects _returnvalue (+ _returnvalue (* _returnvalue_2 5e+02)) (Utilities|Array|MakeArray "ObjectTypeQuery9") true 0 "ForOneFrame"))
      (if _returnvalue_3
        (if (== "/Game/FogOfWar/MaskingActor_BP.MaskingActor_BP_C" (Utilities|GetClass (.HitActor (Collision|BreakHitResult _outhit))))
          (bind _asmasking_actor_bp (Utilities|Casting|CastToMaskingActor_BP (.HitActor (Collision|BreakHitResult _outhit))))
          (Default|AddFogHole _asmasking_actor_bp _outhit))))))

(event Input|MouseEvents|LeftMouseButton
  (params (Key :type Key%20Structure))
  (bind _array (Utilities|Array|MakeArray "ObjectTypeQuery7"))
  (bind (_hitresult _returnvalue) (Class|PlayerController|GetHitResultUnderCursorforObjects _array true))
  (:Released
    (Networking|SwitchHasAuthority
      (:Remote
        (if (Variables|Default|GetPossessedCamera)
          (CallFunction|ReleaseCamera)
          (Variables|Default|SetPossessedCamera false)
          (elif _returnvalue
            (bind _asroom_trigger_bp (Utilities|Casting|CastToRoomTrigger_BP (.HitActor (Collision|BreakHitResult _hitresult))))
            (CallFunction|PossessCameraInroom (Variables|/Script/PCGTesting.RoomTriggerBox|GetroomNum _asroom_trigger_bp) (Variables|/Script/PCGTesting.RoomTriggerBox|GetfloorNum _asroom_trigger_bp))
            (Variables|Default|SetPossessedCamera true)))))))

(fn ConstructionScript)