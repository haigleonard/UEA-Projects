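; Actor that renders one level of a building as instanced floor, room, wall and ceiling meshes.
; Add events append world-space instances to each ISM component, with ceilings raised 300 units and yawed 180 degrees.
; When the player pawn is not the first-person character, it swaps in flat-named color materials shortly after BeginPlay.
; In that case Tick also sets floor, room and wall visibility from MyGameStateBase by FloorNum, leaving ceilings untouched.
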(event EventBeginPlay
  (Utilities|FlowControl|Delay 0.2)
  (Utilities|Casting|CastToFP_FirstPersonCharacter (Game|Player|GetPlayerPawn 0)
    (:CastFailed
      (Rendering|Material|SetMaterial (Variables|Default|GetWallISMComponent) 0 "/Game/Bomb/BombParts/Materials/Black_Mat.Black_Mat")
      (Rendering|Material|SetMaterial (Variables|Default|GetRoomISMComponent) 0 "/Game/darkGreen_Mat.darkGreen_Mat")
      (Rendering|Material|SetMaterial (Variables|Default|GetFloorISMComponent) 0 "/Game/darkGreen_Mat.darkGreen_Mat"))))

(event Collision|EventActorBeginOverlap
  (params (OtherActor :type Actor%20Object%20Reference)))

(event EventTick
  (params (DeltaSeconds :type Float%20%28single-precision%29))
  (Utilities|Casting|CastToFP_FirstPersonCharacter (Game|Player|GetPlayerPawn 0)
    (:CastFailed
      (bind _asmy_game_state_base (Utilities|Casting|CastToMyGameStateBase (Game|GetGameState)))
      (bind _returnvalue (Class|MyGameStateBase|GetFloorVisibility _asmy_game_state_base (Variables|Default|GetfloorNum)))
      (Rendering|SetVisibility (Variables|Default|GetFloorISMComponent) _returnvalue false)
      (Rendering|SetVisibility (Variables|Default|GetRoomISMComponent) _returnvalue false)
      (Rendering|SetVisibility (Variables|Default|GetWallISMComponent) _returnvalue false))))

(event EventAddFloorInstance
  (params (transform :type Transform))
  (Class|InstancedStaticMeshComponent|AddInstanceWorldSpace (Variables|Default|GetFloorISMComponent) transform))

(event EventAddCeilingInstance
  (params (transform :type Transform))
  (bind (_location _rotation _scale) (Math|Transform|BreakTransform transform))
  (bind (_x _y _z) (Math|Vector|BreakVector _location))
  (Class|InstancedStaticMeshComponent|AddInstanceWorldSpace (Variables|Default|GetCeilingISMComponent) (Math|Transform|MakeTransform (Math|Vector|MakeVector _x _y (+ _z 3e+02)) (Math|Rotator|CombineRotators _rotation "180.000000, 0, 0") _scale)))

(event EventAddRoomInstance
  (params (transform :type Transform))
  (Class|InstancedStaticMeshComponent|AddInstanceWorldSpace (Variables|Default|GetRoomISMComponent) transform))

(event EventAddWallInstance
  (params (transform :type Transform))
  (Class|InstancedStaticMeshComponent|AddInstanceWorldSpace (Variables|Default|GetWallISMComponent) transform))

(fn ConstructionScript)