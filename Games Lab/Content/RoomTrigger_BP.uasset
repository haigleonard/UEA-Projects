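; RoomTrigger_BP is a room trigger that reports the closest CCTV camera with line of sight to it and is active only while its floor is visible.
; Each Tick it reads its floor's visibility from MyGameStateBase and switches its collision between query-only and off.
; GetClosestCamera line-traces to every CCTV_BP, ignoring characters and lockers, then caches the nearest camera hit for later calls.
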(event EventBeginPlay)

(event Collision|EventActorBeginOverlap
  (params (OtherActor :type Actor%20Object%20Reference)))

(event EventTick
  (params (DeltaSeconds :type Float%20%28single-precision%29))
  (bind _collisioncomponent (Variables|Default|GetCollisionComponent))
  (bind _asmy_game_state_base (Utilities|Casting|CastToMyGameStateBase (Game|GetGameState)))
  (bind _returnvalue (Class|MyGameStateBase|GetFloorVisibility _asmy_game_state_base (Variables|Default|GetfloorNum)))
  (if _returnvalue
    (Collision|SetCollisionEnabled _collisioncomponent "QueryOnly")
    (else
      (Collision|SetCollisionEnabled _collisioncomponent "NoCollision"))))

(fn ConstructionScript)

(fn GetClosestCamera
  (if (Variables|Default|GetclosestCameraFound)
    _
    (else
      (Variables|Default|SetclosestDistance -1.0)
      (bind _outactors (Actor|GetAllActorsOfClass "/Script/PCGTesting.TP_ThirdPersonCharacter"))
      (bind _output_get (Variables|Default|SetignoreActorArray _outactors))
      (bind _outactors_2 (Actor|GetAllActorsOfClass "/Game/Mannequin/Assets/LockerBP.LockerBP_C"))
      (Utilities|Array|AppendArray _output_get _outactors_2)
      (bind _outactors_3 (Actor|GetAllActorsOfClass "/Game/Geometry/CCTV/CCTV_BP.CCTV_BP_C"))
      (for _array_element _outactors_3
        (bind (_outhit _returnvalue) (Collision|LineTraceByChannel (Transformation|GetActorLocation) (Transformation|GetActorLocation _array_element) "TraceTypeQuery1" true (Variables|Default|GetignoreActorArray) "None"))
        (if _returnvalue
          (bind _ascctv_bp (Utilities|Casting|CastToCCTV_BP (.HitActor (Collision|BreakHitResult _outhit))))
          (if (< (Variables|Default|GetclosestDistance) 0.0)
            (Variables|Default|SetclosestCamera _ascctv_bp :!label _label)
            (Variables|Default|SetclosestDistance (Transformation|GetDistanceTo _ascctv_bp))
            (elif (< (Transformation|GetDistanceTo _ascctv_bp) (Variables|Default|GetclosestDistance))
              (goto _label)))))
      (Variables|Default|SetclosestCameraFound true)))
  (return (Variables|Default|GetclosestCamera)))